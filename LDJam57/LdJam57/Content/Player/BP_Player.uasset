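; Player pawn for a fish-collecting game: it creates the HUD on possession, spawns fish and earns Money from fish it overlaps.
; A Tick countdown spawns random fish classes around the world's vertical axis near the player's height, each with a random goal.
; Maximum fish size scales exponentially with a value derived from the player's Z.
; Holding IA_Fire runs the BP_Vacuum child actor.
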(event `self.ReceivePossessed`
  (params (NewController :type "Controller Object Reference"))
  (bind _asplayer_controller (cast `PlayerController` NewController))
  (bind _returnvalue (`|CreateWidget` "/Game/HUD/BP_HUD.BP_HUD_C" _asplayer_controller))
  (`UserWidget.AddToViewport` _returnvalue 0))

(event `self.ReceiveTick`
  (params (DeltaSeconds :type "Float (single-precision)"))
  (bind (_returnvalue_x _returnvalue_y _returnvalue_z) (`KismetMathLibrary.BreakVector` (`self.K2_GetActorLocation`)))
  (bind (_returnvalue_x_2 _returnvalue_y_2 _returnvalue_z_2) (`KismetMathLibrary.BreakVector` (`self.K2_GetActorLocation`)))
  (bind _fishtospawn (`self.FishToSpawn`))
  (bind (_returnvalue_x_3 _returnvalue_y_3) (`KismetMathLibrary.BreakVector` (* (`KismetMathLibrary.Normal` (`KismetMathLibrary.MakeVector` (`KismetMathLibrary.RandomFloatInRange` -1.0 1.0) (`KismetMathLibrary.RandomFloatInRange` -1.0 1.0))) (750.0 750.0 0.0))))
  (bind (_returnvalue_x_4 _returnvalue_y_4) (`KismetMathLibrary.BreakVector` (* (`KismetMathLibrary.Normal` (`KismetMathLibrary.MakeVector` (`KismetMathLibrary.RandomFloatInRange` -1.0 1.0) (`KismetMathLibrary.RandomFloatInRange` -1.0 1.0))) (750.0 750.0 0.0))))
  (bind _output_get (set `self.currentSpawnTimer` (- (`self.currentSpawnTimer`) DeltaSeconds)))
  (if (<= _output_get 0.0)
    (set `self.currentSpawnTimer` (`self.spawnTimer`))
    (bind _returnvalue (`|SpawnActorFromClass` (`|GetArrayItem` _fishtospawn (`KismetMathLibrary.RandomIntegerInRange` 0 (- (`KismetArrayLibrary.Array_Length` _fishtospawn) 1))) (`KismetMathLibrary.MakeTransform` (`KismetMathLibrary.MakeVector` _returnvalue_x_4 _returnvalue_y_4 (+ (* (- (`KismetMathLibrary.RandomFloat`) 0.5) 1000.0) _returnvalue_z_2))) "Undefined" "MultiplyWithRoot" null null))
    (`/Engine/EditorBlueprintResources/StandardMacros.IsValid` _returnvalue
      (:`Is Valid`
        (bind _result (`/Engine/EditorBlueprintResources/StandardMacros.NegateFloat` _returnvalue_z_2)
          (:`  `
            (`/Game/NPC/BP_Fish.setGoal` _returnvalue (`KismetMathLibrary.MakeVector` _returnvalue_x_3 _returnvalue_y_3 (+ (* (- (`KismetMathLibrary.RandomFloat`) 0.5) 1000.0) _returnvalue_z)) (`KismetMathLibrary.RandomFloatInRange` 0.1 (`KismetMathLibrary.MultiplyMultiply_FloatFloat` 2.0 (/ _result 10000.0))))))))))

(event `self.ReceiveActorBeginOverlap`
  (params (OtherActor :type "Actor Object Reference"))
  (bind _asbp_fish (cast `/Game/NPC/BP_Fish` OtherActor))
  (bind _value (`/Game/NPC/BP_Fish.collect` _asbp_fish))
  (set `self.money` (+ _value (`self.money`))))

(event `EnhancedInput|/Game/input/IA_Fire`
  (params (ActionValue :type Boolean) (ElapsedSeconds :type "Float (double-precision)") (TriggeredSeconds :type "Float (double-precision)") (InputAction :type "InputAction Object Reference" :default "/Game/input/IA_Fire.IA_Fire"))
  (bind _childactor (`ChildActorComponent.ChildActor` (`self.ChildActor`)))
  (:`Started`
    (bind _asbp_vacuum (cast `/Game/Player/BP_Vacuum` _childactor))
    (`/Game/Player/BP_Vacuum.ToggleVacuum` _asbp_vacuum true))
  (:`Completed`
    (bind _asbp_vacuum_2 (cast `/Game/Player/BP_Vacuum` _childactor))
    (`/Game/Player/BP_Vacuum.ToggleVacuum` _asbp_vacuum_2 false)))

(fn `UserConstructionScript`)