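; Player vacuum actor that sucks BP_Fish toward itself.
; ToggleVacuum switches the Cone's query collision and the suck particle emitter together, and starts disabled on BeginPlay.
; Actor overlaps add and remove fish from a tracked array and set their getting-sucked state.
; Each tick steers tracked fish toward the vacuum through movement input and drops invalid entries from the array.
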(event `self.ReceiveBeginPlay`
  (`self.ToggleVacuum` false))

(event `self.ReceiveActorBeginOverlap`
  (params (OtherActor :type "Actor Object Reference"))
  (bind _asbp_fish (cast `/Game/NPC/BP_Fish` OtherActor))
  (`KismetArrayLibrary.Array_AddUnique` (`self.Fish`) _asbp_fish)
  (`/Game/NPC/BP_Fish.setGettingSucked` _asbp_fish true)
  (`KismetSystemLibrary.PrintString` "added fish"))

(event `self.ReceiveActorEndOverlap`
  (params (OtherActor :type "Actor Object Reference"))
  (bind _asbp_fish (cast `/Game/NPC/BP_Fish` OtherActor))
  (`KismetArrayLibrary.Array_RemoveItem` (`self.Fish`) _asbp_fish)
  (`/Game/NPC/BP_Fish.setGettingSucked` _asbp_fish false)
  (`KismetSystemLibrary.PrintString` "removed fish"))

(event `self.ReceiveTick`
  (params (DeltaSeconds :type "Float (single-precision)"))
  (for _array_element (`self.Fish`)
    (`/Engine/EditorBlueprintResources/StandardMacros.IsValid` _array_element
      (:`Is Valid`
        (`Pawn.AddMovementInput` _array_element (`KismetMathLibrary.Normal` (- (`self.K2_GetActorLocation`) (`SceneComponent.K2_GetComponentLocation` (`/Game/NPC/BP_Fish.Sphere` _array_element)))) 1.0 false))
      (:`Is Not Valid`
        (`KismetArrayLibrary.Array_RemoveItem` (`self.Fish`) _array_element)))))

(fn `ToggleVacuum`
  (params (enable :type Boolean))
  (bind _cone (`self.Cone`))
  (bind _ns_suck (`self.NS_Suck`))
  (if enable
    (`PrimitiveComponent.SetCollisionEnabled` _cone "QueryOnly")
    (`FXSystemComponent.SetEmitterEnable` _ns_suck "suck" true)
    (else
      (`PrimitiveComponent.SetCollisionEnabled` _cone "NoCollision")
      (`FXSystemComponent.SetEmitterEnable` _ns_suck "suck" false))))

(fn `UserConstructionScript`)