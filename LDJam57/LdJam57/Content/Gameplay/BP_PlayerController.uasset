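; BP_PlayerController is the player controller that toggles the pause menu through the IA_Pause Enhanced Input action.
; It starts in game-only input; on IA_Pause completion it either creates a BP_HUDPause widget, shows the cursor and switches to game-and-UI input, or removes it and restores game-only input.
; An IsMenuOpen flag tracks the state, and the game itself is never set paused here.
; IncreaseMaxDepth is an empty stub.
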(event `self.ReceiveBeginPlay`
  (`WidgetBlueprintLibrary.SetInputMode_GameOnly` self))

(event `EnhancedInput|/Game/input/IA_Pause`
  (params (ActionValue :type Boolean) (ElapsedSeconds :type "Float (double-precision)") (TriggeredSeconds :type "Float (double-precision)") (InputAction :type "InputAction Object Reference" :default "/Game/input/IA_Pause.IA_Pause"))
  (:`Completed`
    (if (`self.isMenuOpen`)
      (`Widget.RemoveFromParent` (`self.pauseMenu`))
      (set `self.isMenuOpen` false)
      (set `self.bShowMouseCursor` false)
      (`WidgetBlueprintLibrary.SetInputMode_GameOnly` self)
      (else
        (bind _returnvalue (`|CreateWidget` "/Game/HUD/BP_HUDPause.BP_HUDPause_C"))
        (`UserWidget.AddToViewport` _returnvalue 0)
        (bind _output_get (set `self.pauseMenu` _returnvalue))
        (set `self.isMenuOpen` true)
        (set `self.bShowMouseCursor` true)
        (`WidgetBlueprintLibrary.SetInputMode_GameAndUIEx` self _output_get "DoNotLock" false)))))

(fn `increaseMaxDepth`)

(fn `UserConstructionScript`)